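; BP_Book1 is an interactable book actor that shows or hides a WB_Book widget on screen when used.
; Interface events toggle the mesh's custom depth on focus and route interaction to InteractOnServer, which flips InteractToggle.
; That variable's OnRep creates the widget and adds it to the viewport, or calls garbage collection and removes it, so display follows replicated state rather than the interacting player.
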(event Custom|InteractOnServer
  (Variables|Default|SetInteractToggle (not (Variables|Default|GetInteractToggle))))

(event EventBeginPlay)

(event Collision|EventActorBeginOverlap
  (params (OtherActor :type Actor%20Object%20Reference)))

(event EventTick
  (params (DeltaSeconds :type Float%20%28single-precision%29)))

(event EventInterfaceToggleFocus
  (params (Focus :type Boolean))
  (Rendering|SetRenderCustomDepth (Variables|Default|GetBook) Focus))

(event EventInterfaceInteract
  (CallFunction|InteractonServer))

(fn ConstructionScript)

(fn OnRepInteractToggle
  (if (Variables|Default|GetInteractToggle)
    (bind _returnvalue (UserInterface|CreateWidget "/Game/UI/WidgetInteraction/vehicles_ui/WB_Book.WB_Book_C"))
    (bind _output_get (Variables|Default|SetBookInfo _returnvalue))
    (UserInterface|Viewport|AddtoViewport _output_get 0)
    (else
      (Utilities|Platform|CollectGarbage)
      (Widget|RemovefromParent _output_get))))

(fn GetInteractionWidgetRef
  (return (Variables|Default|GetWidgetInteraction)))