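; BP_CPP_Deer is an interactable deer actor that shows or hides an info widget when used.
; Interface events toggle custom depth rendering on the mesh for focus and route interaction to InteractOnServer, which flips InterractToggle.
; The toggle's RepNotify creates WB_DearInfo and adds it to the viewport, or runs garbage collection and removes it.
; GetInteractionWidgetRef exposes the actor's Widget.
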(event Custom|InteractOnServer
  (Variables|Default|SetInterractToggle (not (Variables|Default|GetInterractToggle))))

(event EventBeginPlay)

(event Collision|EventActorBeginOverlap
  (params (OtherActor :type Actor%20Object%20Reference)))

(event EventInterfaceToggleFocus
  (params (Focus :type Boolean))
  (Rendering|SetRenderCustomDepth (Variables|Character|GetMesh) Focus))

(event EventInterfaceInteract
  (CallFunction|InteractonServer))

(event EventTick
  (params (DeltaSeconds :type Float%20%28single-precision%29)))

(fn ConstructionScript)

(fn OnRepInterractToggle
  (if (Variables|Default|GetInterractToggle)
    (bind _returnvalue (UserInterface|CreateWidget "/Game/UI/WidgetInteraction/animals_ui/WB_DearInfo.WB_DearInfo_C"))
    (bind _output_get (Variables|Default|SetDeerInfo _returnvalue))
    (UserInterface|Viewport|AddtoViewport _output_get 0)
    (else
      (Utilities|Platform|CollectGarbage)
      (Widget|RemovefromParent _output_get))))

(fn GetInteractionWidgetRef
  (return (Variables|Default|GetWidget)))