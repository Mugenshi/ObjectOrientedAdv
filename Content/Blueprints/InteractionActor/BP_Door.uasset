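; BP_Door is an interactable swinging door that highlights through custom depth on focus and supplies an interaction widget via a getter.
; Interacting calls InteractOnServer, which flips InteractToggle.
; Its RepNotify plays or reverses a timeline that lerps door yaw through 90 degrees, with play rate derived from separate open and close durations.
; The toggle reads inverted: false opens the door, true closes it.
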(event Custom|Open%20Door
  (bind _door_track (Timeline|open%20door%20T Play)
    (:Update
      (Transformation|SetRelativeRotation (Variables|Default|Getdoor) (Math|Rotator|MakeRotator 0.0 0.0 (Math|Float|Lerp 0.0 -9e+01 _door_track)) false false))
    (:Finished
      (Variables|Default|SetInteractToggle (Variables|Default|GetInteractToggle)))))

(event Custom|InteractOnServer
  (Variables|Default|SetInteractToggle (not (Variables|Default|GetInteractToggle))))

(event Custom|Close%20Door
  (bind _door_track (Timeline|open%20door%20T Reverse)
    (:Update
      (Transformation|SetRelativeRotation (Variables|Default|Getdoor) (Math|Rotator|MakeRotator 0.0 0.0 (Math|Float|Lerp 0.0 -9e+01 _door_track)) false false))
    (:Finished
      (Variables|Default|SetInteractToggle (Variables|Default|GetInteractToggle)))))

(event EventBeginPlay)

(event Collision|EventActorBeginOverlap
  (params (OtherActor :type Actor%20Object%20Reference)))

(event EventTick
  (params (DeltaSeconds :type Float%20%28single-precision%29)))

(event EventInterfaceToggleFocus
  (params (Focus :type Boolean))
  (Rendering|SetRenderCustomDepth (Variables|Default|Getdoor) Focus))

(event EventInterfaceInteract
  (CallFunction|InteractonServer))

(fn ConstructionScript)

(fn OnRepInteractToggle
  (bind _open_door_t (Variables|Default|Getopen%20door%20T))
  (if (not (Variables|Default|GetInteractToggle))
    (Components|Timeline|SetPlayRate _open_door_t (/ 1.0 (Variables|Default|Gettime%20to%20open)))
    (CallFunction|OpenDoor)
    (else
      (Components|Timeline|SetPlayRate _open_door_t (/ 1.0 (Variables|Default|Gettime%20to%20close)))
      (CallFunction|CloseDoor))))

(fn GetInteractionWidgetRef
  (return (Variables|Default|GetWidgetInteraction)))