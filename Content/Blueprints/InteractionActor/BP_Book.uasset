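; BP_Book is an interactable book actor that opens and closes a WB_Book info widget on screen.
; Interface events toggle the mesh's custom depth on focus and pass interaction to InteractOnServer, which flips InteractToggle.
; The toggle's RepNotify creates the widget or removes it with a garbage collection call, without any local-player check.
; It also exposes its interaction widget through a getter.
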(event Custom|InteractOnServer
  (Variables|Default|Setinteract%20Toggle (not (Variables|Default|Getinteract%20Toggle))))

(event EventBeginPlay)

(event Collision|EventActorBeginOverlap
  (params (OtherActor :type Actor%20Object%20Reference)))

(event EventTick
  (params (DeltaSeconds :type Float%20%28single-precision%29)))

(event EventInterfaceInteract
  (CallFunction|InteractonServer))

(event EventInterfaceToggleFocus
  (params (Focus :type Boolean))
  (Rendering|SetRenderCustomDepth (Variables|Default|GetSM_Book_03) Focus))

(fn ConstructionScript)

(fn OnRepInteractToggle
  (if (Variables|Default|Getinteract%20Toggle)
    (bind _returnvalue (UserInterface|CreateWidget "/Game/UI/WidgetInteraction/vehicles_ui/WB_Book.WB_Book_C"))
    (bind _output_get (Variables|Default|SetBookInfo _returnvalue))
    (UserInterface|Viewport|AddtoViewport _output_get 0)
    (else
      (Utilities|Platform|CollectGarbage)
      (Widget|RemovefromParent _output_get))))

(fn GetInteractionWidgetRef
  (return (Variables|Default|GetWidgetInteraction)))