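; BP_lamp1 is an interactable lamp actor whose point light toggles on and off.
; Interface events highlight the lamp through custom depth on focus and route interaction to InteractOnServer, which flips InteractToggle.
; The InteractToggle RepNotify sets the light's visibility to match the state.
; A getter exposes the lamp's interaction widget.
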(event Custom|InteractOnServer
  (Variables|Default|SetInteractToggle (not (Variables|Default|GetInteractToggle))))

(event EventBeginPlay)

(event Collision|EventActorBeginOverlap
  (params (OtherActor :type Actor%20Object%20Reference)))

(event EventTick
  (params (DeltaSeconds :type Float%20%28single-precision%29)))

(event EventInterfaceToggleFocus
  (params (Focus :type Boolean))
  (Rendering|SetRenderCustomDepth (Variables|Default|Getlamp) Focus))

(event EventInterfaceInteract
  (CallFunction|InteractonServer))

(fn ConstructionScript)

(fn OnRepInteractToggle
  (if (Variables|Default|GetInteractToggle)
    (Rendering|SetVisibility (Variables|Default|GetPointLight) true false)
    (else
      (Rendering|SetVisibility (Variables|Default|GetPointLight) false false))))

(fn GetInteractionWidgetRef
  (return (Variables|Default|GetWidgetInteraction)))