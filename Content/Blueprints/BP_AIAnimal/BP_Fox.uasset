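; BP_Fox is an AI animal Blueprint that makes a fox wander around the level.
; On BeginPlay it starts roaming at once, setting a slow walk speed and using AI MoveTo toward a random reachable navmesh point around its current location.
; Each successful move triggers the next decision after a random delay of a few seconds, forming a loop.
; A failed move has no handler, so the roaming stops.
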(event Custom|Decide%20next%20action
  (params (Skip%20Delay? :type Boolean))
  (if Skip%20Delay?
    _
    (else
      (Utilities|FlowControl|Delay (Math|Conversions|ToFloat(Integer) (Math|Random|RandomIntegerinRange 1 5)))))
  (CallFunction|RandomRoam))

(event Custom|Random%20Roam
  ;[1 1 1] Racndom Roam
  (Variables|/Script/Engine.CharacterMovementComponent|SetMaxWalkSpeed (Variables|Character|GetCharacterMovement) 1.5e+02)
  (AI|AIMoveTo self (.RandomLocation (AI|Navigation|GetRandomReachablePointinRadius (Transformation|GetActorLocation) 1.5e+03 0 0)) 0 5.0 false
    (:OnSuccess
      (CallFunction|DecideNextAction false))))

(event EventBeginPlay
  (CallFunction|DecideNextAction true))

(fn ConstructionScript)